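; BP_Npc03 is an AI-driven NPC character that senses physical contact and reacts to attacks.
; Capsule hits are reported to AI touch perception at the NPC's own location.
; The IFAttack event plays a forward death montage and sets the BBDamage blackboard key to false as it starts.
; The IsPlayAinm flag blocks retriggering until the montage completes or is interrupted.
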(event OnComponentHit(CapsuleComponent)
  (params (HitComponent :type Primitive%20Component%20Object%20Reference) (OtherActor :type Actor%20Object%20Reference) (OtherComp :type Primitive%20Component%20Object%20Reference) (NormalImpulse :type Vector :default "0, 0, 0") (Hit :type Hit%20Result%20Structure%20%28by%20ref%29))
  (Class|AISenseTouch|ReportTouchEvent self OtherActor (Transformation|GetActorLocation)))

(event EventBeginPlay
  (|CallParentFunction) ; This node is disabled and will not be called.\nDrag off pins to build functionality.
)

(event Collision|EventActorBeginOverlap
  (params (OtherActor :type Actor%20Object%20Reference))
  (|CallParentFunction OtherActor) ; This node is disabled and will not be called.\nDrag off pins to build functionality.
)

(event EventTick
  (params (DeltaSeconds :type Float%20%28single-precision%29))
  (|CallParentFunction DeltaSeconds) ; This node is disabled and will not be called.\nDrag off pins to build functionality.
)

(event EventIFAttack
  (if (Variables|Default|GetIsPlayAinm)
    (Animation|Montage|PlayMontage (Variables|Character|GetMesh) "/Game/BTProject/CHAR/NPC/Anim/Death_Fwd_Montage.Death_Fwd_Montage"
      (:then
        (Variables|Default|SetIsPlayAinm false)
        (AI|Components|Blackboard|SetValueasBool (AI|GetBlackboard 0) (Utilities|Name|MakeLiteralName "BBDamage") false))
      (:OnCompleted
        (Variables|Default|SetIsPlayAinm true :!label _label))
      (:OnInterrupted
        (goto _label)))))

(fn ConstructionScript
  (|CallParentFunction))