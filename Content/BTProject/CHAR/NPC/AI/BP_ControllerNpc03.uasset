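; AI controller for NPC 03 that runs BT_Npc03 on BeginPlay and feeds player perception into its Blackboard.
; Target perception updates branch by sense: sight sets or clears the target object, while sight, hearing and damage write BBLocation.
; Sensed damage also sets BBDamage, which is never reset here.
; The touch branch is empty, and general perception updates just print actor names.
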(event OnPerceptionUpdated(AIPerception)
  (params (UpdatedActors :type Array%20of%20Actor%20Object%20References))
  (for _array_element UpdatedActors
    (Development|PrintString (Utilities|GetDisplayName _array_element))))

(event OnTargetPerceptionUpdated(AIPerception)
  (params (Actor :type Actor%20Object%20Reference) (Stimulus :type AI%20Stimulus%20Structure))
  (bind (_age _expirationage _strength _stimuluslocation _receiverlocation _tag _bsuccessfullysensed) (Utilities|Struct|BreakAIStimulus Stimulus))
  (bind (_age_2 _expirationage_2 _strength_2 _stimuluslocation_2 _receiverlocation_2 _tag_2 _bsuccessfullysensed_2) (Utilities|Struct|BreakAIStimulus Stimulus))
  (bind _returnvalue (Class|AIPerceptionSystem|GetSenseClassforStimulus Stimulus))
  (if (== Actor (Game|GetPlayerCharacter 0))
    (Utilities|FlowControl|Sequence
      (:then_0
        (if (== _returnvalue "/Script/AIModule.AISense_Sight")
          (AI|Components|Blackboard|SetValueasObject (Variables|Default|GetBlackboard) (Variables|Default|GetKey%20Name) (Utilities|SelectObject (Game|GetPlayerCharacter 0) 0 _bsuccessfullysensed_2))
          (AI|Components|Blackboard|SetValueasVector (Variables|Default|GetBlackboard) (Utilities|Name|MakeLiteralName "BBLocation") _stimuluslocation_2)))
      (:then_1
        (if (== _returnvalue "/Script/AIModule.AISense_Hearing")
          (AI|Components|Blackboard|SetValueasVector (Variables|Default|GetBlackboard) (Utilities|Name|MakeLiteralName "BBLocation") (.StimulusLocation (Utilities|Struct|BreakAIStimulus Stimulus)))))
      (:then_2
        (if (== _returnvalue "/Script/AIModule.AISense_Damage")
          (AI|Components|Blackboard|SetValueasVector (Variables|Default|GetBlackboard) (Utilities|Name|MakeLiteralName "BBLocation") _stimuluslocation)
          (if _bsuccessfullysensed
            (AI|Components|Blackboard|SetValueasBool (Variables|Default|GetBlackboard) (Utilities|Name|MakeLiteralName "BBDamage") true))))
      (:then_3
        (if (== _returnvalue "/Script/AIModule.AISense_Touch")
          _)))))

(event EventBeginPlay
  (AI|RunBehaviorTree "/Game/BTProject/CHAR/NPC/AI/BT/BT_Npc03.BT_Npc03"))

(event EventTick
  (params (DeltaSeconds :type Float%20%28single-precision%29)))

(fn ConstructionScript)